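; Test actor that exercises item stack creation and amount changes using the health potion item.
; On BeginPlay it constructs a stack with itself as Outer, stores it in ItemStack, then prints the amount before and after calling AddToAmount.
; GetInteger and SetInteger, despite their names, read and write ItemStack; a disconnected variant of the test modifies the stack through the getter.
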(event Collision|EventActorBeginOverlap
  (params (OtherActor :type Actor%20Object%20Reference)))

(event EventTick
  (params (DeltaSeconds :type Float%20%28single-precision%29)))

(event EventBeginPlay
  (bind _stack (CallFunction|ConstructItemStackfromClass "/Game/Dynamic/Inventory/Items/Item_HealthPotion.Item_HealthPotion_C" 4 self))
  (bind _output_get (Variables|Default|SetItemStack _stack))
  (Development|PrintString (Utilities|String|ToString(Integer) (Variables|/Script/AbilitySystemProject.ItemStack|GetAmount _output_get)) true true "(R=0.000000,G=0.660000,B=1.000000,A=1.000000)" 2e+01)
  (Class|ItemStack|AddtoAmount _stack 300)
  (Development|PrintString (Utilities|String|ToString(Integer) (Variables|/Script/AbilitySystemProject.ItemStack|GetAmount (Variables|Default|GetItemStack))) true true "(R=0.000000,G=0.660000,B=1.000000,A=1.000000)" 2e+01))

(fn ConstructionScript)

(fn GetInteger
  (return (Variables|Default|GetItemStack)))

(fn SetInteger
  (params (Stack :type Item%20Stack%20Object%20Reference))
  (Variables|Default|SetItemStack Stack))