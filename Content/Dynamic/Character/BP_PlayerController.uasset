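; Player controller that owns the ability HUD and in-game status menu, linking input to the Gameplay Ability System.
; Five slot inputs look up the HUD slot's ability class, activate it on the controlled character and update its targeting and combo state.
; Abilities are added to HUD slots through events, and cooldowns are matched to slots by ability class.
; The menu input toggles a status screen fed by the character's attribute set, switching input mode and cursor.
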(event Custom|UpdateAbilityIconCooldown
  (params (GAInstance :type Gameplay%20Ability%20Base%20Object%20Reference) (CooldownDuration :type Float%20%28single-precision%29))
  (bind _returnvalue (Class|GameplayAbilityBase|GetAbilityInfo GAInstance))
  (for _array_element (Variables|/Game/Dynamic/UI/WBP_HUD.WBP_HUD_C|GetSlots (Variables|Default|GetHUD))
    (if (== (.abilityclass (Variables|/Game/Dynamic/UI/WBP_AbilityIcon.WBP_AbilityIcon_C|GetAbilityInfo _array_element)) (.abilityclass _returnvalue))
      (Default|SetMaxCooldown _array_element CooldownDuration)
      (Default|StartCooldown _array_element))))

(event EventBeginPlay
  (bind _returnvalue (UserInterface|CreateWidget "/Game/Dynamic/UI/WBP_HUD.WBP_HUD_C"))
  (bind _output_get (Variables|Default|SetHUD _returnvalue))
  (UserInterface|Viewport|AddtoViewport _output_get 0)
  (bind _asbp_character_base (Utilities|Casting|CastToBP_CharacterBase (Pawn|GetControlledPawn)))
  (Variables|Default|SetCharacterBase _asbp_character_base))

(event EventTick
  (params (DeltaSeconds :type Float%20%28single-precision%29)))

(event EventAddAbilitytoUI
  (params (AbilityInfo :type Gameplay%20Ability%20Info%20Structure) (AbilityInstance :type Gameplay%20Ability%20Base%20Object%20Reference))
  (Default|AddAbilitytoSlot (Variables|Default|GetHUD) AbilityInfo AbilityInstance))

(event EventPossess
  (params (PossessedPawn :type Pawn%20Object%20Reference))
  (Game|Player|SetViewTargetwithBlend PossessedPawn 0.0 "VTBlend_Linear" 0.0 false))

(event Input|ActionEvents|InputActionOpenInGameMenu
  (params (Key :type Key%20Structure :default "None"))
  (:Pressed
    (bind _ingamemenu (Variables|Default|GetInGameMenu)
      (:then
        (CallFunction|RemoveinGameMenu _ingamemenu))
      (:else
        (bind _returnvalue (UserInterface|CreateWidget "/Game/Dynamic/UI/WBP_StatusScreen.WBP_StatusScreen_C" self))
        (Variables|Default|SetInGameMenu _returnvalue)
        (bind _characterbase (Variables|Default|GetCharacterBase)
          (:then
            (Default|SetAttributeSet _returnvalue (Variables|/Script/AbilitySystemProject.ProjectCharacter|GetAttributeSetBase _characterbase))
            (Input|SetInputModeGameandUI self _returnvalue "DoNotLock" true)
            (Variables|Default|SetbShowMouseCursor true)
            (UserInterface|Viewport|AddtoViewport _returnvalue 0))
          (:else))))))

(event Input|ActionEvents|InputActionSlotOneAbility
  (params (Key :type Key%20Structure :default "None"))
  (:Pressed
    (CallFunction|TryActivateAbilityinUISlot)))

(event Input|ActionEvents|InputActionSlotTwoAbility
  (params (Key :type Key%20Structure :default "None"))
  (:Pressed
    (CallFunction|TryActivateAbilityinUISlot 1)))

(event Input|ActionEvents|InputActionSlotThreeAbility
  (params (Key :type Key%20Structure :default "None"))
  (:Pressed
    (CallFunction|TryActivateAbilityinUISlot 2)))

(event Input|ActionEvents|InputActionSlotFourAbility
  (params (Key :type Key%20Structure :default "None"))
  (:Pressed
    (CallFunction|TryActivateAbilityinUISlot 3)))

(event Input|ActionEvents|InputActionSlotFiveAbility
  (params (Key :type Key%20Structure :default "None"))
  (:Pressed
    (CallFunction|TryActivateAbilityinUISlot 4)))

(fn ConstructionScript)

(fn TryActivateAbilityinUISlot
  (params (SlotNumber :type Integer))
  (bind (_isvalid _class) (Default|GetSlotAbilityClass (Variables|Default|GetHUD) SlotNumber))
  (if _isvalid
    (bind _asbp_character_base (Utilities|Casting|CastToBP_CharacterBase (Pawn|GetControlledPawn)))
    (Utilities|IsValid (Ability|GetAbilitySystemComponent _asbp_character_base)
      (:Is%20Valid
        (Abilities|TryActivateAbilitybyClass (Ability|GetAbilitySystemComponent _asbp_character_base) _class true)
        (Utilities|Casting|CastToBP_GameplayAbilityBase_TargetTypeClass _class
          (:then
            (Variables|/Game/Dynamic/Character/BP_CharacterBase.BP_CharacterBase_C|SetIsTargeting _asbp_character_base true))
          (:CastFailed
            (Variables|/Game/Dynamic/Character/BP_CharacterBase.BP_CharacterBase_C|SetIsTargeting _asbp_character_base false)))
        (Class|AbilitySystemComponent|TargetCancel (Ability|GetAbilitySystemComponent _asbp_character_base))
        (Class|ProjectCharacter|EndCombo _asbp_character_base)))))

(fn RemoveinGameMenu
  (params (WidgetToRemove :type Widget%20Object%20Reference))
  (Widget|RemovefromParent WidgetToRemove)
  (Input|SetInputModeGameOnly self)
  (Variables|Default|SetbShowMouseCursor false)
  (Variables|Default|SetInGameMenu 0))

(fn RemoveAllWidgets
  (Viewport|RemoveAllWidgets)
  (Input|SetInputModeGameOnly self)
  (Variables|Default|SetbShowMouseCursor false)
  (Variables|Default|SetInGameMenu 0))