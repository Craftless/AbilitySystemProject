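; Melee character base Blueprint that picks the attack montage for a three-step melee combo.
; DetermineCombo copies the combo counter into the damage level and uses it to select a montage from the montage array.
; The counter advances after each pick and wraps back to the first step after the third hit.
; The event graph and construction script add no logic of their own.
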(event EventBeginPlay
  (|CallParentFunction) ; This node is disabled and will not be called.\nDrag off pins to build functionality.
)

(event Collision|EventActorBeginOverlap
  (params (OtherActor :type Actor%20Object%20Reference)))

(fn ConstructionScript
  (|CallParentFunction))

(fn DetermineCombo
  (bind _output_get (Variables|Default|SetMeleeDamageLevel (Variables|Default|GetMeleeComboCount)))
  (switch int (Variables|Default|GetMeleeComboCount)
    (:Default
      (Variables|Default|SetMeleeMontage (Utilities|Array|Get(acopy) (Variables|Default|GetMeleeMontages) (- _output_get 1)) :!label _label)
      (Math|Integer|IncrementInt (Variables|Default|GetMeleeComboCount) :!label _label_2))
    (:1
      (goto _label))
    (:2
      (Variables|Default|SetMeleeMontage (Utilities|Array|Get(acopy) (Variables|Default|GetMeleeMontages) (- _output_get 1)))
      (goto _label_2))
    (:3
      (Variables|Default|SetMeleeMontage (Utilities|Array|Get(acopy) (Variables|Default|GetMeleeMontages) (- _output_get 1)))
      (Variables|Default|SetMeleeComboCount 1))))