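; Gameplay ability that lets a character use an inventory item.
; On activation it waits for one item-use gameplay event, carrying the item and an optional montage, and cancels itself after a fixed delay.
; It plays any montage, then executes the item's use on the character and ends, or cancels if interrupted or no item is supplied.
; On end, any stored item is notified of success or cancellation.
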(event Ability|EventActivateAbility
  (Ability|CommitAbility)
  (bind _payload (Ability|Tasks|WaitGameplayEvent "(TagName=\"inventory.item.use\")" 0 true)
    (:then
      (Utilities|FlowControl|Delay 1e+01)
      (Ability|CancelAbility))
    (:EventReceived
      (bind _asanim_montage (Utilities|Casting|CastToAnimMontage (.optionalobject2 _payload))
        (:then
          (|PlayMontageandWaitProxy "None" _asanim_montage 1.0 "None" true 1.0 0.0
            (:OnCompleted
              (bind _asitem (Utilities|Casting|CastToItem (.optionalobject _payload) :!label _label)
                (:then
                  (Variables|Default|SetItem _asitem)
                  (bind _characterbase (CallFunction|GetCharacterBaseandController))
                  (Class|Item|ExecuteUse _asitem _characterbase)
                  (Ability|EndAbility))
                (:CastFailed
                  (Ability|CancelAbility))))
            (:OnBlendOut
              (goto _label))
            (:OnInterrupted
              (Ability|CancelAbility :!label _label_2))
            (:OnCancelled
              (goto _label_2))))
        (:CastFailed
          (goto _label))))))

(event Ability|EventOnEndAbility
  (params (bWasCancelled :type Boolean))
  (bind _returnvalue (not bWasCancelled))
  (bind _item (Variables|Default|GetItem)
    (:then
      (Default|CallFonFinishedUsing _item _returnvalue)
      (Development|PrintString (Utilities|String|ToString(Boolean) _returnvalue) true true "(R=0.306199,G=1.000000,B=0.000000,A=1.000000)"))
    (:else)))