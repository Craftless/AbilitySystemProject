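; BP_Item appears to be a base inventory item for character use, with Gameplay Ability System effect support.
; UseItem shows a potion mesh on the character's Item component, and ExecuteUse clears it.
; GetEffectSpecToApply returns no spec, apparently as a default for child items.
; GetSpecForAttrAddition builds an outgoing effect spec with a tag-keyed SetByCaller magnitude, adding a duration for regeneration effects.
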(event EventExecuteUse
  (params (User :type Project%20Character%20Object%20Reference))
  (bind _asbp_character_base (Utilities|Casting|CastToBP_CharacterBase User))
  (Components|StaticMesh|SetStaticMesh (Variables|/Game/Dynamic/Character/BP_CharacterBase.BP_CharacterBase_C|GetItem _asbp_character_base) 0))

(event EventUseItem
  (params (User :type Project%20Character%20Object%20Reference))
  (bind _asbp_character_base (Utilities|Casting|CastToBP_CharacterBase User))
  (Components|StaticMesh|SetStaticMesh (Variables|/Game/Dynamic/Character/BP_CharacterBase.BP_CharacterBase_C|GetItem _asbp_character_base) "/Game/Dynamic/Pickups/Models/potion_01.potion_01"))

(fn GetEffectSpectoApply
  (params (ASC :type Ability%20System%20Component%20Object%20Reference))
  (return false ""))

(fn GetSpecforAttrAddition
  (params (ASC :type Ability%20System%20Component%20Object%20Reference) (GameplayEffectClass :type Gameplay%20Effect%20Class%20Reference) (DataTag :type Gameplay%20Tag%20Structure) (Magnitude :type Float%20%28single-precision%29) (IsRegen :type Boolean) (Duration :type Float%20%28single-precision%29))
  (bind _returnvalue (Ability|GameplayEffect|AssignTagSetbyCallerMagnitude (GameplayEffects|MakeOutgoingSpec :self ASC :GameplayEffectClass GameplayEffectClass) DataTag Magnitude))
  (if IsRegen
    (Ability|GameplayEffect|SetDuration _returnvalue Duration))
  (return _returnvalue))