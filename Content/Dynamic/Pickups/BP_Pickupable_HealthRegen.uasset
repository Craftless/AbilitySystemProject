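; Health pickup that heals the actor interacting with it through the Gameplay Ability System.
; On interact it runs the parent logic, then builds a GE_AddHealth spec on that actor's ability system component.
; HealAmount is passed in as a set-by-caller magnitude under the health add tag, and the spec is applied to that same actor.
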(event EventBeginPlay
  (|CallParentFunction) ; This node is disabled and will not be called.\nDrag off pins to build functionality.
)

(event Collision|EventActorBeginOverlap
  (params (OtherActor :type Actor%20Object%20Reference))
  (|CallParentFunction OtherActor) ; This node is disabled and will not be called.\nDrag off pins to build functionality.
)

(event EventTick
  (params (DeltaSeconds :type Float%20%28single-precision%29))
  (|CallParentFunction DeltaSeconds) ; This node is disabled and will not be called.\nDrag off pins to build functionality.
)

(fn ConstructionScript
  (|CallParentFunction))

(fn OnInteract
  (params (OtherActor :type Actor%20Object%20Reference))
  (bind _returnvalue (Ability|GetAbilitySystemComponent OtherActor))
  (|CallParentFunction OtherActor)
  (bind _returnvalue_2 (Ability|GameplayEffect|AssignTagSetbyCallerMagnitude (GameplayEffects|MakeOutgoingSpec :self _returnvalue :GameplayEffectClass "/Game/Dynamic/GameplayAbilities/General/Attributes/GE_AddHealth.GE_AddHealth_C") "(TagName=\"attributes.health.add\")" (Variables|Default|GetHealAmount)))
  (GameplayEffects|ApplyGameplayEffectSpecToSelf _returnvalue _returnvalue_2))