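; A pickupable item actor that a character collects into their inventory by interacting with it.
; OnInteract asks the BP_CharacterBase for an active spacious inventory, using a stack built from ItemClass and Amount, then destroys the actor if adding succeeds.
; GetItemStack supplies the stack to add, either built the same way or taken from StackToAdd, depending on UseQuickInitInstead.
; A debug print of max stack size runs before the add.
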(event EventBeginPlay
  (|CallParentFunction) ; This node is disabled and will not be called.\nDrag off pins to build functionality.
)

(event Collision|EventActorBeginOverlap
  (params (OtherActor :type Actor%20Object%20Reference))
  (|CallParentFunction OtherActor) ; This node is disabled and will not be called.\nDrag off pins to build functionality.
)

(event EventTick
  (params (DeltaSeconds :type Float%20%28single-precision%29))
  (|CallParentFunction DeltaSeconds) ; This node is disabled and will not be called.\nDrag off pins to build functionality.
)

(fn ConstructionScript
  (|CallParentFunction))

(fn OnInteract
  (params (OtherActor :type Actor%20Object%20Reference))
  (|CallParentFunction OtherActor)
  (bind _asbp_character_base (Utilities|Casting|CastToBP_CharacterBase OtherActor))
  (bind _stack (CallFunction|ConstructItemStackfromClass (Variables|Default|GetItemClass) (Variables|Default|GetAmount)))
  (bind _array_element (Default|GetActiveSpaciousInventory _asbp_character_base _stack))
  (Utilities|IsValid _array_element
    (:Is%20Valid
      (bind _stack_2 (CallFunction|GetItemStack))
      (Development|PrintString (Utilities|String|ToString(Integer) (.maxstacksize (Variables|/Script/AbilitySystemProject.Item|GetItemInfo (Variables|/Script/AbilitySystemProject.ItemStack|GetItem _stack_2)))) true true "(R=0.912338,G=0.000000,B=1.000000,A=1.000000)")
      (bind _returnvalue (Class|Inventory|AddItemStacktoSlots _array_element _stack_2))
      (if _returnvalue
        (Actor|DestroyActor)))))

(fn GetItemStack
  (if (Variables|Default|GetUseQuickInitInstead)
    (bind _stack (CallFunction|ConstructItemStackfromClass (Variables|Default|GetItemClass) (Variables|Default|GetAmount)))
    (return _stack)
    (else
      (return (Variables|Default|GetStackToAdd)))))