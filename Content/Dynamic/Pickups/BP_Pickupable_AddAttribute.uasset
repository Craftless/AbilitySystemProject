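; Pickup Blueprint that modifies an attribute on the interacting actor through the Gameplay Ability System, then destroys itself.
; On interact, it builds a spec from a configurable Gameplay Effect class and passes the amount as a tagged SetByCaller magnitude.
; When flagged as regen, it also overrides the spec's duration before applying it to that actor's ability system component.
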(event Collision|EventActorBeginOverlap
  (params (OtherActor :type Actor%20Object%20Reference))
  (|CallParentFunction OtherActor) ; This node is disabled and will not be called.\nDrag off pins to build functionality.
)

(fn ConstructionScript
  (|CallParentFunction))

(fn OnInteract
  (params (OtherActor :type Actor%20Object%20Reference))
  (bind _returnvalue (Ability|GetAbilitySystemComponent OtherActor))
  (|CallParentFunction OtherActor)
  (bind _returnvalue_2 (Ability|GameplayEffect|AssignTagSetbyCallerMagnitude (GameplayEffects|MakeOutgoingSpec :self _returnvalue :GameplayEffectClass (Variables|Default|GetGameplay%20Effect%20Class)) (Variables|Default|GetSetByCallerTag) (Variables|Default|GetAmount)))
  (if (Variables|Default|GetIsRegen)
    (Ability|GameplayEffect|SetDuration _returnvalue_2 (Variables|Default|GetDuration)))
  (GameplayEffects|ApplyGameplayEffectSpecToSelf _returnvalue _returnvalue_2)
  (Actor|DestroyActor))