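; AI controller for Shinbi that runs its behavior tree and uses perception to choose a hostile enemy.
; Perception updates on hostile actors set or clear the blackboard enemy key along with controller focus.
; Actors on the game mode's exclusion list are ignored, and changes to that list re-evaluate currently seen actors, clearing or restoring the enemy accordingly.
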(event OnTargetPerceptionUpdated(AIPerception)
  (params (Actor :type Actor%20Object%20Reference) (Stimulus :type AI%20Stimulus%20Structure))
  (bind _gamemode (Variables|Default|GetGameMode)
    (:then
      (if (not (Utilities|Array|ContainsItem (Variables|/Game/Dynamic/FirstPersonCPP/Blueprints/BP_AbilitySystemProjectGameMode.BP_AbilitySystemProjectGameMode_C|GetExcludeFromAIPerceptionChecks _gamemode) Actor))
        (CallFunction|UpdatePerception (.bSuccessfullySensed (Utilities|Struct|BreakAIStimulus Stimulus)) Actor :!label _label)))
    (:else
      (goto _label))))

(event Custom|OnExcludeActorsChanged
  (bind _gamemode (Variables|Default|GetGameMode)
    (:then
      (for _array_element (Class|AIPerceptionComponent|GetCurrentlyPerceivedActors (Variables|Default|GetAIPerception) "/Script/AIModule.AISense_Sight")
        (CallFunction|UpdatePerception (not (Utilities|Array|ContainsItem (Variables|/Game/Dynamic/FirstPersonCPP/Blueprints/BP_AbilitySystemProjectGameMode.BP_AbilitySystemProjectGameMode_C|GetExcludeFromAIPerceptionChecks _gamemode) _array_element)) _array_element)))
    (:else)))

(event EventBeginPlay
  (AI|RunBehaviorTree "/Game/Dynamic/AI/BT_Shinbi.BT_Shinbi")
  (bind _blackboardcomponent (Class|AIController|UseBlackboard "/Game/Dynamic/AI/BB_Shinbi.BB_Shinbi"))
  (Variables|Default|SetBlackboardComp _blackboardcomponent)
  (bind _asbp_shinbi (Utilities|Casting|CastToBP_Shinbi (Pawn|GetControlledPawn)))
  (Variables|Default|SetPossessedPawn _asbp_shinbi)
  (bind _asbp_ability_system_project_game_mode (Utilities|Casting|CastToBP_AbilitySystemProjectGameMode (Game|GetGameMode)))
  (bind _output_get (Variables|Default|SetGameMode _asbp_ability_system_project_game_mode))
  (EventDispatchers|BindEventtoOnExcludefromAIPerceptionChanged _output_get (delegate Custom|OnExcludeActorsChanged)))

(event EventTick
  (params (DeltaSeconds :type Float%20%28single-precision%29)))

(fn ConstructionScript)

(fn SetEnemyValue
  (params (ObjectValue :type Actor%20Object%20Reference) (ClearValue :type Boolean))
  (if ClearValue
    (AI|Components|Blackboard|ClearValue (Variables|Default|GetBlackboardComp) (Variables|Default|GetEnemyKey))
    (AI|ClearFocus)
    (else
      (AI|Components|Blackboard|SetValueasObject (Variables|Default|GetBlackboardComp) (Variables|Default|GetEnemyKey) ObjectValue)
      (Class|MagicLeapHMDFunctionLibrary|SetFocusActor ObjectValue true))))

(fn UpdatePerception
  (params (Condition :type Boolean) (ActorToCheck :type Actor%20Object%20Reference))
  (bind _returnvalue (Class|ProjectCharacter|IsOtherActorHostile (Variables|Default|GetPossessedPawn) ActorToCheck))
  (if _returnvalue
    (if Condition
      (CallFunction|SetEnemyValue ActorToCheck false)
      (else
        (CallFunction|SetEnemyValue 0 true)))))