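; Base Gameplay Ability Blueprint that gives abilities shared helpers for cost validation and HUD cooldown display.
; GetCharacterAndController casts the owning actor to BP_Shinbi and its controller to BP_PlayerController, so the helpers are tied to that character.
; DoUICooldown starts the cooldown on HUD slots whose ability class matches this ability's info.
; IsCostStillValid compares the current Health, Mana or Stamina attribute, chosen by cost type, against the absolute cost.
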(fn GetCharacterandController
  (bind _asbp_shinbi (Utilities|Casting|CastToBP_Shinbi (Ability|GetOwningActorfromActorInfo)))
  (bind _asbp_player_controller (Utilities|Casting|CastToBP_PlayerController (Pawn|GetController _asbp_shinbi)))
  (return _asbp_shinbi _asbp_player_controller))

(fn DoUICooldown
  (bind _controller (CallFunction|GetCharacterandController))
  (Utilities|IsValid _controller
    (:Is%20Valid
      (for _array_element (Variables|/Game/Dynamic/UI/WBP_HUD.WBP_HUD_C|GetSlots (Variables|/Game/Dynamic/Character/BP_PlayerController.BP_PlayerController_C|GetHUD _controller))
        (bind _returnvalue (Class|GameplayAbilityBase|GetAbilityInfo))
        (if (== (.abilityclass (Variables|/Game/Dynamic/UI/WBP_AbilityIcon.WBP_AbilityIcon_C|GetAbilityInfo _array_element)) (.abilityclass _returnvalue))
          (Default|StartCooldown _array_element))))))

(fn IsCostStillValid
  (bind _returnvalue (Class|GameplayAbilityBase|GetAbilityInfo))
  (bind _character (CallFunction|GetCharacterandController))
  (bind _attributesetbase (Variables|/Script/AbilitySystemProject.ProjectCharacter|GetAttributeSetBase _character)
    (:then
      (return (>= (Utilities|Select :Index (.costtype _returnvalue) :Health (.currentvalue (Variables|/Script/AbilitySystemProject.AttributeSetBase|GetHealth _attributesetbase)) :Mana (.currentvalue (Variables|/Script/AbilitySystemProject.AttributeSetBase|GetMana _attributesetbase)) :Stamina (.currentvalue (Variables|/Script/AbilitySystemProject.AttributeSetBase|GetStamina _attributesetbase))) (Math|Float|Absolute(Float) (.cost _returnvalue)))))
    (:else
      (return false))))