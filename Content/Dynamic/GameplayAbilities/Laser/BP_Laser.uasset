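; Laser beam actor for a gameplay ability that tracks hostile characters at its end point and requests damage on them.
; Each tick it stretches the beam by feeding the end trigger's distance, minus the initial length, into the anim instance's end-bone offset.
; Trigger overlaps maintain a hostile target list, filtered through the instigator.
; A looping timer sends that list to the instigator as target data in a deal-damage gameplay event.
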(event OnComponentBeginOverlap(LaserEndTrigger)
  (params (OverlappedComponent :type Primitive%20Component%20Object%20Reference) (OtherActor :type Actor%20Object%20Reference) (OtherComp :type Primitive%20Component%20Object%20Reference) (OtherBodyIndex :type Integer) (bFromSweep :type Boolean) (SweepResult :type Hit%20Result%20Structure%20%28by%20ref%29))
  (bind _asproject_character (Utilities|Casting|CastToProjectCharacter OtherActor))
  (bind _asproject_character_2 (Utilities|Casting|CastToProjectCharacter (Game|GetInstigator)))
  (bind _returnvalue (Class|ProjectCharacter|IsOtherActorHostile _asproject_character_2 _asproject_character))
  (if _returnvalue
    (Utilities|Array|AddUnique (Variables|Default|GetOverlappingActors) _asproject_character)))

(event OnComponentEndOverlap(LaserEndTrigger)
  (params (OverlappedComponent :type Primitive%20Component%20Object%20Reference) (OtherActor :type Actor%20Object%20Reference) (OtherComp :type Primitive%20Component%20Object%20Reference) (OtherBodyIndex :type Integer))
  (bind _asproject_character (Utilities|Casting|CastToProjectCharacter OtherActor))
  (Utilities|Array|RemoveItem (Variables|Default|GetOverlappingActors) _asproject_character))

(event Custom|SendDealDamageEvent
  (Ability|SendGameplayEventtoActor (Game|GetInstigator) "(TagName=\"ability.laser.dealdamage\")" (Utilities|Struct|MakeGameplayEventData "(TagName=\"ability.laser.dealdamage\")" 0 0 0 0 "()" "(GameplayTags=)" "(GameplayTags=)" 0.0 (Ability|TargetData|AbilityTargetDatafromActorArray (Variables|Default|GetOverlappingActors)))))

(event EventBeginPlay
  (Variables|Default|SetInitialBeamLength (Math|Vector|VectorLength (- (Transformation|GetSocketLocation (Variables|Default|GetLaserMesh) "end") (Transformation|GetActorLocation))))
  (bind _asabp_laser_beam (Utilities|Casting|CastToABP_LaserBeam (Components|SkeletalMesh|GetAnimInstance (Variables|Default|GetLaserMesh))))
  (Variables|Default|SetLaserBeamAnimInstance _asabp_laser_beam)
  (Utilities|Time|SetTimerbyEvent (delegate Custom|SendDealDamageEvent) 0.2 true))

(event EventTick
  (params (DeltaSeconds :type Float%20%28single-precision%29))
  (bind _laserbeamaniminstance (Variables|Default|GetLaserBeamAnimInstance)
    (:then
      (Variables|/Game/Dynamic/GameplayAbilities/Laser/ABP_LaserBeam.ABP_LaserBeam_C|SetEndBoneOffset _laserbeamaniminstance (Math|Vector|MakeVector (- (Math|Vector|VectorLength (- (Transformation|GetWorldLocation (Variables|Default|GetLaserEndTrigger)) (Transformation|GetActorLocation))) (Variables|Default|GetInitialBeamLength)) 0.0 0.0)))
    (:else)))

(fn ConstructionScript)