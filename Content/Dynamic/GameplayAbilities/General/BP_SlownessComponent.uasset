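; BP_SlownessComponent is a gameplay ability component that temporarily slows a character by lowering its CharacterMovement MaxWalkSpeed.
; On BeginPlay it reduces the speed by SlownessAmount, either as a fraction or a flat value depending on IsPercentage.
; After a Duration delay it applies the inverse operation to the current speed rather than restoring a cached original.
; The component does not remove itself afterwards, and Tick is unused.
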(event EventBeginPlay
  (bind _slownessamount (Variables|Default|GetSlownessAmount))
  (bind _charactermovement (Variables|Default|GetCharacterMovement))
  (bind _output_get (Variables|/Script/Engine.CharacterMovementComponent|SetMaxWalkSpeed _charactermovement (select (Variables|Default|GetIsPercentage) (* (Variables|/Script/Engine.CharacterMovementComponent|GetMaxWalkSpeed _charactermovement) (- 1.0 (Variables|Default|GetSlownessAmount))) (- (Variables|/Script/Engine.CharacterMovementComponent|GetMaxWalkSpeed _charactermovement) (Variables|Default|GetSlownessAmount)))))
  (Utilities|FlowControl|Delay (Variables|Default|GetDuration))
  (Variables|/Script/Engine.CharacterMovementComponent|SetMaxWalkSpeed _charactermovement (select (Variables|Default|GetIsPercentage) (/ _output_get (- 1.0 _slownessamount)) (+ _output_get _slownessamount))))

(event EventTick
  (params (DeltaSeconds :type Float%20%28single-precision%29)))