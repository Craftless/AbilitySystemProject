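; GA_GrantExperience is a Gameplay Ability that grants a fixed amount of experience to an actor named in a gameplay event.
; On activation it waits for the grant-experience event, but ends itself after a short delay, leaving a brief listening window.
; When the event arrives, it applies GE_GrantExperience to the payload's Target with a set-by-caller magnitude, then ends.
; Debug prints mark activation and effect application.
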(event Ability|EventActivateAbility
  (Development|PrintString "DSOPAJSOF" true true "(R=0.680996,G=0.000000,B=1.000000,A=1.000000)")
  (bind _payload (Ability|Tasks|WaitGameplayEvent "(TagName=\"attributes.experience.grantexperience\")" 0)
    (:then
      (Utilities|FlowControl|Delay 0.2)
      (Ability|EndAbility))
    (:EventReceived
      (bind _returnvalue (Ability|GameplayEffect|AssignTagSetbyCallerMagnitude (Ability|MakeOutgoingGameplayEffectSpec "/Game/Dynamic/GameplayAbilities/General/Experience/GE_GrantExperience.GE_GrantExperience_C") "(TagName=\"attributes.experience.grantexperience\")" 1.5e+02))
      (GameplayEffects|ApplyGameplayEffectSpecToTarget _returnvalue (Ability|TargetData|AbilityTargetDatafromActor (.Target (Utilities|Struct|BreakGameplayEventData _payload))))
      (Development|PrintString "Applied Effect" true true "(R=0.000000,G=1.000000,B=0.170386,A=1.000000)")
      (Ability|EndAbility))))

(event Ability|EventOnEndAbility
  (params (bWasCancelled :type Boolean)))